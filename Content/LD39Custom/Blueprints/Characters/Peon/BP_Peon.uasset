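; BP_Peon is a selectable unit that receives orders from the player through the GM_LD39 game mode.
; On BeginPlay it binds to the game mode's clear-selection and action dispatchers, with selection state stored as a flag and shown by a decal.
; When an action fires, a selected peon copies the game mode's last location and target into its AI blackboard.
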(event Custom|ActionEvent
  (CallFunction|OnActionRecieved))

(event Custom|ClearSelectionDispatcher_Event_0
  (CallFunction|SetSelection false))

(event EventBeginPlay
  (Utilities|FlowControl|Sequence
    (:then_0
      (bind _asgm_ld39 (Utilities|Casting|CastToGM_LD39 (Game|GetGameMode)))
      (EventDispatchers|AssignClearSelectionDispatcher _asgm_ld39 (delegate Custom|ClearSelectionDispatcher_Event_0)))
    (:then_1
      (bind _asgm_ld39_2 (Utilities|Casting|CastToGM_LD39 (Game|GetGameMode)))
      (EventDispatchers|AssignActionDispatcher _asgm_ld39_2 (delegate Custom|ActionEvent)))))

(event Collision|EventActorBeginOverlap
  (params (OtherActor :type Actor%20Object%20Reference)))

(event EventSetSelection
  (params (Selection :type Boolean))
  (Rendering|SetVisibility (Variables|Default|GetDecal) Selection false)
  (Variables|Default|SetSelected Selection))

(event EventTick
  (params (DeltaSeconds :type Float%20%28single-precision%29)))

(fn ConstructionScript)

(fn OnActionRecieved
  (if (Variables|Default|GetSelected)
    (bind _asgm_ld39 (Utilities|Casting|CastToGM_LD39 (Game|GetGameMode)))
    (Utilities|FlowControl|Sequence
      (:then_0
        ;[1 1 1] Location
        (AI|Components|Blackboard|SetValueasVector (AI|GetBlackboard self) (Variables|Default|GetLocationKeyname) (Variables|/Game/LD39Custom/Blueprints/Logic/GM_LD39.GM_LD39_C|GetLastLocation _asgm_ld39)))
      (:then_1
        ;[1 1 1] Target
        (AI|Components|Blackboard|SetValueasObject (AI|GetBlackboard self) (Variables|Default|GetTargetKeyName) (Variables|/Game/LD39Custom/Blueprints/Logic/GM_LD39.GM_LD39_C|GetLastTarget _asgm_ld39))))))

(fn GetSelection
  (return (Variables|Default|GetSelected)))