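; PC_CameraRig is the player controller for the RTS camera rig, turning mouse clicks into game-wide commands.
; Right press traces under the cursor on Visibility and, on a hit, stores the location and actor on GM_LD39, then calls its action dispatcher.
; Left release calls the game mode's clear-selection dispatcher.
; The game mode acts as the hub, so the controller holds no unit logic.
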(event EventBeginPlay)

(event EventTick
  (params (DeltaSeconds :type Float%20%28single-precision%29)))

(event Input|MouseEvents|RightMouseButton
  (params (Key :type Key%20Structure :default "AnyKey"))
  (bind (_hitresult _returnvalue) (Game|Player|GetHitResultUnderCursorbyChannel "TraceTypeQuery1" true))
  (bind (_bblockinghit _binitialoverlap _time _location _impactpoint _normal _impactnormal _physmat _hitactor) (Collision|BreakHitResult _hitresult))
  (:Pressed
    (if _returnvalue
      (bind _asgm_ld39 (Utilities|Casting|CastToGM_LD39 (Game|GetGameMode)))
      (Variables|/Game/LD39Custom/Blueprints/Logic/GM_LD39.GM_LD39_C|SetLastLocation _asgm_ld39 _location)
      (Variables|/Game/LD39Custom/Blueprints/Logic/GM_LD39.GM_LD39_C|SetLastTarget _asgm_ld39 _hitactor)
      (Default|CallActionDispatcher _asgm_ld39))))

(event Input|MouseEvents|CtrlLeftMouseButton
  (params (Key :type Key%20Structure :default "AnyKey")))

(event Input|MouseEvents|LeftMouseButton
  (params (Key :type Key%20Structure :default "AnyKey"))
  (:Released
    (bind _asgm_ld39 (Utilities|Casting|CastToGM_LD39 (Game|GetGameMode)))
    (Default|CallClearSelectionDispatcher _asgm_ld39)))

(fn ConstructionScript)